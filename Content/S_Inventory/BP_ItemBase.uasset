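; BP_ItemBase is an inventory item actor that sets up its data and label widget from an item ID.
; On BeginPlay it spawns a separate BP_ItemData actor at its own transform as a data container and keeps a reference to it.
; When Table_ItemData has a row matching ItemID, it copies the ID, name, icon and size into that container.
; It then passes the data and itself to the widget component's label.
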(event `self.ReceiveBeginPlay`
  (`self.InitByItemID`))

(fn `InitByItemID`
  (bind _bp_itemdata (`self.BP_ItemData`))
  (bind _returnvalue (`|SpawnActorFromClass` "/Game/S_Inventory/BP_ItemData.BP_ItemData_C" (`self.GetTransform` self) "AlwaysSpawn" "MultiplyWithRoot" null null))
  (set `self.BP_ItemData` _returnvalue)
  (bind _returnvalue_2 (`|GetDataTableRow` "/Game/S_Inventory/DataTable/Table_ItemData.Table_ItemData" (`self.ItemID`))
    (:`then`
      (set `/Game/S_Inventory/BP_ItemData.ID` (`self.ItemID`) _bp_itemdata)
      (bind (_name _icon _size) (break `/Game/S_Inventory/DataTable/Struct/ST_ItemData` _returnvalue_2))
      (set `/Game/S_Inventory/BP_ItemData.Name` _name _bp_itemdata)
      (set `/Game/S_Inventory/BP_ItemData.Icon` _icon _bp_itemdata)
      (set `/Game/S_Inventory/BP_ItemData.Size` _size _bp_itemdata)
      (message `/Game/S_Inventory/BPI/BPI_Item.InitLabelUI` (`WidgetComponent.GetWidget` (`self.Widget`)) (`self.BP_ItemData`) self))))

(fn `UserConstructionScript`)